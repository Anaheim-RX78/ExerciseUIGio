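; Turret enemy that fires projectiles at the first-person character within range and can be destroyed by damage.
; Tick sets CanShoot from distance alone and rotates the barrel toward the player only when an in-range visibility trace hits nothing.
; A looping timer, its interval randomized once at BeginPlay, spawns damage-carrying projectiles along the barrel's rotation.
; TakeDamage pushes health percentage to the widget health bar and destroys the turret at zero.
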(event `self.ReceiveBeginPlay`
  (bind _returnvalue (`GameplayStatics.GetActorOfClass` "/Game/FirstPerson/Blueprints/BP_FirstPersonCharacter.BP_FirstPersonCharacter_C"))
  (set `self.AsCharacter` _returnvalue)
  (`KismetSystemLibrary.K2_SetTimerDelegate` (delegate `Shoot`) (`KismetMathLibrary.RandomFloatInRange` 1.0 3.0) true)
  (bind _aswbp_health_bar (cast `/Game/UI/WBp_HealthBar` (`WidgetComponent.GetWidget` (`self.Widget`))))
  (set `self.As WBp Health Bar` _aswbp_health_bar)
  (`/Game/BpI_Health.ResetHealth`))

(event `Shoot`
  (if (`self.CanShoot`)
    (`|SpawnActorFromClass` "/Game/FirstPerson/Blueprints/BP_FirstPersonProjectile.BP_FirstPersonProjectile_C" (`KismetMathLibrary.MakeTransform` (`SceneComponent.K2_GetComponentLocation` (`self.Scene`)) (`SceneComponent.K2_GetComponentRotation` (`self.Cylinder1`)) (0.8 0.8 0.8)) "Undefined" "MultiplyWithRoot" null (`self.Damage`) null)))

(event `self.ReceiveTick`
  (params (DeltaSeconds :type "Float (single-precision)"))
  (bind _cylinder1 (`self.Cylinder1`))
  (bind _returnvalue (`SceneComponent.K2_GetComponentLocation` (`self.Scene`)))
  (bind _returnvalue_2 (`self.K2_GetActorLocation` (`self.AsCharacter`)))
  (bind _returnvalue_3 (<= (`KismetMathLibrary.Vector_Distance` _returnvalue _returnvalue_2) 800.0))
  (set `self.CanShoot` _returnvalue_3)
  (if _returnvalue_3
    (bind (_outhit _returnvalue_4) (`KismetSystemLibrary.LineTraceSingle` :`Start` _returnvalue :`End` _returnvalue_2 :`TraceChannel` "TraceTypeQuery1" :`DrawDebugType` "ForOneFrame"))
    (if (not _returnvalue_4)
      (`SceneComponent.K2_SetWorldRotation` _cylinder1 (`KismetMathLibrary.FindLookAtRotation` (`SceneComponent.K2_GetComponentLocation` _cylinder1) (`self.K2_GetActorLocation` (`self.AsCharacter`))) false false))))

(event `/Game/BpI_Health.ResetHealth`
  (set `self.CurrentHealth` (`self.MaxHealth`)))

(event `/Game/BpI_Health.Death`
  (`self.K2_DestroyActor`))

(fn `GetPercent`
  (params (MaxHealth :type "Float (double-precision)") (Currenthealth :type "Float (double-precision)"))
  (returns (Percent :type "Float (double-precision)"))
  (return (/ Currenthealth MaxHealth)))

(fn `TakeDamage`
  (params (Amount :type "Float (double-precision)"))
  (returns (NewHealth :type "Float (double-precision)"))
  (bind _returnvalue (- (`self.CurrentHealth`) Amount))
  (bind _percent (`/Game/BpI_Health.GetPercent` (`self.MaxHealth`) _returnvalue))
  (`/Game/UI/WBp_HealthBar.OnPercentChange` (`self.As WBp Health Bar`) _percent)
  (if (<= _returnvalue 0.0)
    (`/Game/BpI_Health.Death`)
    (return 0.0)
    (else
      (bind _output_get (set `self.CurrentHealth` _returnvalue))
      (return _output_get))))

(fn `UserConstructionScript`)